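; BP_HD_Player is the player character Blueprint that lets the player cling to objects through BPClingComponent.
; F sphere-traces forward and passes the hit actor to the component to cling, or unclings if already attached.
; While clinging, move input follows directions the component computes from control rotation; this graph adds no movement otherwise.
; Cling interface events relay enter and exit to the AnimInstance and pass flailing back to the component.
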(event Input|EnhancedActionEvents|EnhancedInputActionIA_Player_Move
  (params (ActionValue :type Vector%202D%20Structure) (ElapsedSeconds :type Float%20%28double-precision%29) (TriggeredSeconds :type Float%20%28double-precision%29) (InputAction :type Input%20Action%20Object%20Reference :default "/Game/CHJ/Input/IA_Player_Move.IA_Player_Move"))
  (bind _returnvalue (Pawn|GetControlRotation :!class /Script/Engine.Pawn))
  (bind _returnvalue_2 (Pawn|GetControlRotation :!class /Script/Engine.Pawn))
  (bind _bp_clingcomponent (Variables|Default|GetBP_ClingComponent))
  (bind _returnvalue_3 (Math|Vector|GetForwardVector (Math|Rotator|MakeRotator 0.0 0.0 (.yaw _returnvalue))))
  (bind _returnvalue_4 (Math|Vector|GetRightVector (Math|Rotator|MakeRotator (.roll _returnvalue_2) 0.0 (.yaw _returnvalue_2))))
  (bind (_forwardworlddirection _rightworlddirection) (Default|CalculatePawnInputDirection _bp_clingcomponent _returnvalue_3 _returnvalue_4))
  (if (Variables|/Game/ClingingComponent/Blueprints/Components/BP_ClingComponent.BP_ClingComponent_C|GetClinging? (Variables|Default|GetBP_ClingComponent))
    (Pawn|Input|AddMovementInput _rightworlddirection (.x ActionValue) false)
    (Pawn|Input|AddMovementInput _forwardworlddirection (.y ActionValue) false)))

(event EventBeginPlay
  (Default|SetupClingComponent (Variables|Default|GetBP_ClingComponent) self (Variables|Default|GetCapsuleComponent) (Variables|Character|GetMesh)))

(event Collision|EventActorBeginOverlap
  (params (OtherActor :type Actor%20Object%20Reference)))

(event EventOnClingFlail
  (params (Flail? :type Boolean))
  ;[1 0.6654 0.2106] Interface Events
  (Default|HandleFlail (Variables|Default|GetBP_ClingComponent) Flail?))

(event EventOnClingEnter
  ;[1 0.6654 0.2106] Interface Events
  (Class|BPIClingComponent|OnClingAnimation(Message) (Components|SkeletalMesh|GetAnimInstance (Variables|Character|GetMesh)) true))

(event EventTick
  (params (DeltaSeconds :type Float%20%28single-precision%29)))

(event EventOnClingExit
  ;[1 0.6654 0.2106] Interface Events
  (Class|BPIClingComponent|OnClingAnimation(Message) (Components|SkeletalMesh|GetAnimInstance (Variables|Character|GetMesh)) false))

(event EventOnClingReset
  ;[1 0.6654 0.2106] Interface Events
)

(event Input|KeyboardEvents|E
  (params (Key :type Key%20Structure :default "None"))
  ;[1 1 1] Try and cling to an object, and try and grasp to the current clingobject / 물체에 달라붙으려고 노력하고, 현재 붙어 있는 물체를 붙잡으려고 노력하세요.
)

(event Input|KeyboardEvents|T
  (params (Key :type Key%20Structure :default "None")))

(event Input|KeyboardEvents|F
  (params (Key :type Key%20Structure :default "None"))
  (bind _returnvalue (Transformation|GetActorLocation))
  (bind _bp_clingcomponent (Variables|Default|GetBP_ClingComponent))
  ;[1 1 1] Try and cling to an object, and try and grasp to the current clingobject / 물체에 달라붙으려고 노력하고, 현재 붙어 있는 물체를 붙잡으려고 노력하세요.
  (:Pressed
    (if (Variables|/Game/ClingingComponent/Blueprints/Components/BP_ClingComponent.BP_ClingComponent_C|GetClinging? _bp_clingcomponent)
      ;;[1 0.6654 0.2106] Handles Clinging and unclinging / 매달림과 풀림을 처리합니다.
      (Default|TryUnclingto _bp_clingcomponent)
      (else
        (bind (_outhit _returnvalue_2) (Collision|SphereTraceByChannel _returnvalue (+ _returnvalue (* (Transformation|GetActorForwardVector) 3e+02)) 5.0 (Variables|/Game/ClingingComponent/Blueprints/Components/BP_ClingComponent.BP_ClingComponent_C|GetTrace%20Channel _bp_clingcomponent) false (Actor|GetAllChildActors true) "ForDuration"))
        (if _returnvalue_2
          (Default|TryClingto (Variables|Default|GetBP_ClingComponent) (.HitActor (Collision|BreakHitResult _outhit)) _outhit))))))

(fn ConstructionScript)