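; Test actor that attaches a nearby pawn to its Cube through a physics constraint when the 0 key is pressed.
; The key runs a debug-drawn sphere trace for Pawn objects at the actor's location and constrains the Cube to the hit component, passing "pelvis" as the Cube-side bone name.
; Tick is empty, and leftover forward-movement and constraint nodes are unconnected.
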(event EventBeginPlay)

(event Collision|EventActorBeginOverlap
  (params (OtherActor :type Actor%20Object%20Reference)))

(event EventTick
  (params (DeltaSeconds :type Float%20%28single-precision%29)))

(event Input|KeyboardEvents|8
  (params (Key :type Key%20Structure :default "None")))

(event Input|KeyboardEvents|0
  (params (Key :type Key%20Structure :default "None"))
  (bind _returnvalue (Transformation|GetActorLocation))
  (:Pressed
    (bind (_outhit _returnvalue_2) (Collision|SphereTraceForObjects _returnvalue _returnvalue 1.2e+02 (Utilities|Array|MakeArray "ObjectTypeQuery3") false 0 "ForDuration"))
    (if _returnvalue_2
      (Class|PhysicsConstraintComponent|SetConstrainedComponents (Variables|Default|GetPhysicsConstraint) (Variables|Default|GetCube) "pelvis" (.HitComponent (Collision|BreakHitResult _outhit)) "None"))))

(fn ConstructionScript)