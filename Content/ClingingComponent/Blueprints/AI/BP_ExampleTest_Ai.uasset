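; Example test AI for the clinging system, acting as a thin host that delegates to BPAIComponent and BPFactionComponent.
; On BeginPlay it gathers its cling objects as the AI component's limbs, sets the default state and enables turning.
; While alive, it routes damage to the faction component's health logic.
; An interface event updates the AI component's cling targets, which are told to uncling when the actor is destroyed.
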(event EventModifyClingCharacters
  (params (Add? :type Boolean) (Actor :type Actor%20Object%20Reference))
  ;[1 0.8064 0.3944] Interface events
  (Default|ModifyClingTargets (Variables|Default|GetBP_AIComponent) Add? Actor))

(event Game|Damage|EventAnyDamage
  (params (Damage :type Float%20%28single-precision%29) (DamageType :type Damage%20Type%20Object%20Reference) (InstigatedBy :type Controller%20Object%20Reference) (DamageCauser :type Actor%20Object%20Reference))
  ;[0.9479 0.7873 0.4295] Damaged
  (if (not (Variables|/Game/ClingingComponent/Blueprints/AI/BP_AIComponent.BP_AIComponent_C|GetDead? (Variables|Default|GetBP_AIComponent)))
    (Default|ModifyHealth (Variables|Default|GetBP_FactionComponent) Damage DamageCauser)))

(event EventDestroyed
  ;[1 1 1] Comment
  (for _array_element (Variables|/Game/ClingingComponent/Blueprints/AI/BP_AIComponent.BP_AIComponent_C|GetClingTargets (Variables|Default|GetBP_AIComponent))
    (Default|TryUnclingto (Actor|GetComponentbyClass _array_element "/Game/ClingingComponent/Blueprints/Components/BP_ClingComponent.BP_ClingComponent_C"))))

(event EventBeginPlay
  ;[1 0.8064 0.3944] BeginPlay
  (Variables|/Game/ClingingComponent/Blueprints/AI/BP_AIComponent.BP_AIComponent_C|SetDefaultState (Variables|Default|GetBP_AIComponent) "NewEnumerator0")
  ;;[1 1 1] Gets all child objects and puts them into an array
  (bind _objects (CallFunction|GetAllClingObjects self))
  (Variables|/Game/ClingingComponent/Blueprints/AI/BP_AIComponent.BP_AIComponent_C|SetAllLimbObjects (Variables|Default|GetBP_AIComponent) _objects)
  (Variables|/Game/ClingingComponent/Blueprints/AI/BP_AIComponent.BP_AIComponent_C|SetTurning (Variables|Default|GetBP_AIComponent) true))

(fn ConstructionScript)