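; BP_Giant_Ai is a climbable giant AI enemy that registers as the player character's Boss while the player is inside its Detection volume.
; BeginPlay caches clingable limb objects in BPAIComponent and seeds targets from overlapping pawns, then Detection overlaps add and remove targets.
; Damage routes to BPFactionComponent for health and, while alive, to the AI component's stun check.
; Clinging characters are tracked through an interface event and released when the giant is destroyed.
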(event OnComponentBeginOverlap(Detection)
  (params (OverlappedComponent :type Primitive%20Component%20Object%20Reference) (OtherActor :type Actor%20Object%20Reference) (OtherComp :type Primitive%20Component%20Object%20Reference) (OtherBodyIndex :type Integer) (bFromSweep :type Boolean) (SweepResult :type Hit%20Result%20Structure%20%28by%20ref%29))
  ;[1 0.8064 0.3944] Detect Enemies
  (bind _asbp_climbing_character (Utilities|Casting|CastToBP_ClimbingCharacter OtherActor)
    (:then
      (if (== _asbp_climbing_character (Game|GetPlayerCharacter 0))
        (Variables|/Game/ClingingComponent/Blueprints/BP_ClimbingCharacter.BP_ClimbingCharacter_C|SetBoss _asbp_climbing_character self)))
    (:CastFailed
      _))
  (Default|TryAddTarget (Variables|Default|GetBP_AIComponent) OtherActor))

(event OnComponentEndOverlap(Detection)
  (params (OverlappedComponent :type Primitive%20Component%20Object%20Reference) (OtherActor :type Actor%20Object%20Reference) (OtherComp :type Primitive%20Component%20Object%20Reference) (OtherBodyIndex :type Integer))
  ;[1 0.8064 0.3944] Detect Enemies
  (bind _asbp_climbing_character (Utilities|Casting|CastToBP_ClimbingCharacter OtherActor)
    (:then
      (if (== _asbp_climbing_character (Game|GetPlayerCharacter 0))
        (Variables|/Game/ClingingComponent/Blueprints/BP_ClimbingCharacter.BP_ClimbingCharacter_C|SetBoss _asbp_climbing_character 0)))
    (:CastFailed
      _))
  (Default|TryRemoveTarget (Variables|Default|GetBP_AIComponent) OtherActor))

(event EventModifyClingCharacters
  (params (Add? :type Boolean) (Actor :type Actor%20Object%20Reference))
  ;[1 0.8064 0.3944] Interface events
  (Default|ModifyClingTargets (Variables|Default|GetBP_AIComponent) Add? Actor))

(event Game|Damage|EventAnyDamage
  (params (Damage :type Float%20%28single-precision%29) (DamageType :type Damage%20Type%20Object%20Reference) (InstigatedBy :type Controller%20Object%20Reference) (DamageCauser :type Actor%20Object%20Reference))
  (bind _bp_factioncomponent (Variables|Default|GetBP_FactionComponent))
  ;[0.9479 0.7873 0.4295] Damaged
  (Default|ModifyHealth _bp_factioncomponent Damage DamageCauser)
  (if (not (Variables|/Game/ClingingComponent/Blueprints/AI/BP_AIComponent.BP_AIComponent_C|GetDead? (Variables|Default|GetBP_AIComponent)))
    (Default|StunCheck (Variables|Default|GetBP_AIComponent) 3.0 Damage (Variables|/Game/ClingingComponent/Blueprints/AI/BP_FactionComponent.BP_FactionComponent_C|GetMaxHealth _bp_factioncomponent))))

(event EventDestroyed
  ;[1 1 1] Comment
  (for _array_element (Variables|/Game/ClingingComponent/Blueprints/AI/BP_AIComponent.BP_AIComponent_C|GetClingTargets (Variables|Default|GetBP_AIComponent))
    (Default|TryUnclingto (Actor|GetComponentbyClass _array_element "/Game/ClingingComponent/Blueprints/Components/BP_ClingComponent.BP_ClingComponent_C"))))

(event EventBeginPlay
  (bind _detection (Variables|Default|GetDetection))
  ;[1 0.8064 0.3944] BeginPlay
  (Variables|/Game/ClingingComponent/Blueprints/AI/BP_AIComponent.BP_AIComponent_C|SetDefaultState (Variables|Default|GetBP_AIComponent) (Variables|-CharacterValues|GetState))
  ;;[1 1 1] Gets all child objects and puts them into an array
  (bind _objects (CallFunction|GetAllClingObjects self))
  (Variables|/Game/ClingingComponent/Blueprints/AI/BP_AIComponent.BP_AIComponent_C|SetAllLimbObjects (Variables|Default|GetBP_AIComponent) _objects)
  ;[1 1 1] Comment
  (bind (_outactors _returnvalue) (Collision|ComponentOverlapActors _detection (Transformation|GetWorldTransform _detection) (Utilities|Array|MakeArray "ObjectTypeQuery3") "/Script/Engine.Pawn" (Utilities|Array|MakeArray self)))
  (if _returnvalue
    (for _array_element _outactors
      (Default|TryAddTarget (Variables|Default|GetBP_AIComponent) _array_element))))

(fn ConstructionScript)