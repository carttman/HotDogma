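; Spider AI enemy pawn that can cling to other characters, wiring cling, AI and faction components together.
; A detection volume adds and removes AI targets on overlap, seeded at BeginPlay with pawns already inside.
; Damage goes to the faction component's health, and hits spawn green blood at the nearest bone.
; Cling enter and exit message the anim instance, and exit also cycles AI targets.
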(event OnComponentBeginOverlap(Detection)
  (params (OverlappedComponent :type Primitive%20Component%20Object%20Reference) (OtherActor :type Actor%20Object%20Reference) (OtherComp :type Primitive%20Component%20Object%20Reference) (OtherBodyIndex :type Integer) (bFromSweep :type Boolean) (SweepResult :type Hit%20Result%20Structure%20%28by%20ref%29))
  ;[1 0.8064 0.3944] Detect Enemies
  (Default|TryAddTarget (Variables|Default|GetBP_AIComponent) OtherActor))

(event OnComponentEndOverlap(Detection)
  (params (OverlappedComponent :type Primitive%20Component%20Object%20Reference) (OtherActor :type Actor%20Object%20Reference) (OtherComp :type Primitive%20Component%20Object%20Reference) (OtherBodyIndex :type Integer))
  ;[1 0.8064 0.3944] Detect Enemies
  (Default|TryRemoveTarget (Variables|Default|GetBP_AIComponent) OtherActor))

(event EventTick
  (params (DeltaSeconds :type Float%20%28single-precision%29)))

(event Game|Damage|EventAnyDamage
  (params (Damage :type Float%20%28single-precision%29) (DamageType :type Damage%20Type%20Object%20Reference) (InstigatedBy :type Controller%20Object%20Reference) (DamageCauser :type Actor%20Object%20Reference))
  ;[0.9479 0.7873 0.4295] Damaged
  (Default|ModifyHealth (Variables|Default|GetBP_FactionComponent) Damage DamageCauser))

(event EventOnClingEnter
  ;[1 1 1] Comment
  (Class|BPIClingComponent|OnClingAnimation(Message) (Components|SkeletalMesh|GetAnimInstance (Variables|Character|GetMesh)) true))

(event Collision|EventActorBeginOverlap
  (params (OtherActor :type Actor%20Object%20Reference)))

(event EventOnClingExit
  ;[1 1 1] Comment
  (Class|BPIClingComponent|OnClingAnimation(Message) (Components|SkeletalMesh|GetAnimInstance (Variables|Character|GetMesh)) false)
  (Default|CycleTargets (Variables|Default|GetBP_AIComponent)))

(event EventBeginPlay
  (bind _detection (Variables|Default|GetDetection))
  ;[1 0.8064 0.3944] BeginPlay
  (Variables|/Game/ClingingComponent/Blueprints/AI/BP_AIComponent.BP_AIComponent_C|SetDefaultState (Variables|Default|GetBP_AIComponent) (Variables|Default|GetState))
  ;;[1 1 1] Gets all child objects and puts them into an array
  (Default|SetupClingComponent (Variables|Default|GetBP_CingComp) self (Variables|Collision|GetCapsuleComponent) (Variables|Character|GetMesh))
  ;[1 1 1] Comment
  (bind (_outactors _returnvalue) (Collision|ComponentOverlapActors _detection (Transformation|GetWorldTransform _detection) (Utilities|Array|MakeArray "ObjectTypeQuery3") "/Script/Engine.Pawn" (Utilities|Array|MakeArray self)))
  (if _returnvalue
    (for _array_element _outactors
      (Default|TryAddTarget (Variables|Default|GetBP_AIComponent) _array_element))))

(event EventOnHitEffect
  (params (Location :type Vector :default "0, 0, 0"))
  ;[1 1 1] Comment
  (Effects|SpawnEmitteratLocation "/Game/ClingingComponent/Effects/P_Hit_Blood_Green.P_Hit_Blood_Green" (.BoneLocation (Class|SkinnedMeshComponent|FindClosestBoneK2 (Variables|Character|GetMesh) Location 0.0)) "0, 0, 0" "0.300000,0.300000,0.300000"))

(fn ConstructionScript)