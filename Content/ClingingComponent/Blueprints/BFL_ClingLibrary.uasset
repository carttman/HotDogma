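; Blueprint function library of helpers for the clinging system, built around BP_ClingComponent and BP_ClingObject_Base actors.
; It reports whether an actor is clinging and to what, and finds cling objects by sphere trace with an attached-or-free filter or among an actor's child actors.
; Other helpers filter objects by group or type, resolve move-to points, and compute turn checks, L/R turn names and facing rotations.
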(fn IsActorClinging?
  (params (Target :type Actor%20Object%20Reference))
  (bind _returnvalue (Actor|GetComponentbyClass Target "/Game/ClingingComponent/Blueprints/Components/BP_ClingComponent.BP_ClingComponent_C"))
  (bind _clinging_ (Variables|/Game/ClingingComponent/Blueprints/Components/BP_ClingComponent.BP_ClingComponent_C|GetClinging? _returnvalue))
  (bind _currentdynamicobject (Variables|/Game/ClingingComponent/Blueprints/Components/BP_ClingComponent.BP_ClingComponent_C|GetCurrentDynamicObject _returnvalue))
  (Utilities|IsValid _returnvalue
    (:Is%20Valid
      (if _clinging_
        (return _clinging_ (Actor|GetParentActor _currentdynamicobject) _currentdynamicobject)
        (else
          _)))
    (:Is%20Not%20Valid
      _))
  (return false 0 0))

(fn GetTurnAngle
  (params (Actor :type Actor%20Object%20Reference) (Location :type Vector%20%28by%20ref%29) (Angle :type Float%20%28single-precision%29))
  (return (> (Math|Float|Absolute(Float) (.yaw (Math|Rotator|Delta(Rotator) (Math|Rotator|FindLookatRotation (Transformation|GetActorLocation Actor) Location) (Transformation|GetActorRotation Actor)))) Angle)))

(fn GetTurnName
  (params (Actor :type Actor%20Object%20Reference) (Target :type Vector%20%28by%20ref%29))
  (bind _returnvalue (Transformation|GetActorLocation Actor))
  (bind _returnvalue_2 (Transformation|GetActorRotation Actor))
  (bind _returnvalue_3 (Math|Rotator|FindLookatRotation _returnvalue Target))
  (bind (_roll _pitch) (Math|Rotator|BreakRotator _returnvalue_2))
  (return (select (> (.yaw (Math|Rotator|Delta(Rotator) _returnvalue_2 _returnvalue_3)) 0.0) "R" "L") (Math|Rotator|MakeRotator _roll _pitch (.Yaw (Math|Rotator|BreakRotator _returnvalue_3)))))

(fn GetClingObjectsGroup
  (params (Objects :type Array%20of%20BP%20Cling%20Object%20Base%20Object%20References) (Group :type Integer))
  (bind _localobjects (LocalVariables|GetLocalObjects))
  (Utilities|Array|Clear _localobjects)
  (for _array_element Objects
    (if (== (Variables|/Game/ClingingComponent/Blueprints/Components/BP_ClingObject_Base.BP_ClingObject_Base_C|GetClingObjectGroup _array_element) Group)
      (Utilities|Array|Add _localobjects _array_element)))
  (return (LocalVariables|GetLocalObjects)))

(fn GetClingObjectsType
  (params (Objects :type Array%20of%20BP%20Cling%20Object%20Base%20Object%20References) (Type :type E_ClingDamageType%20Enum :default "NewEnumerator0"))
  (bind _localobjects (LocalVariables|GetLocalObjects))
  (Utilities|Array|Clear _localobjects)
  (for _array_element Objects
    (if (Utilities|Enum|Equal(Enum) (Variables|/Game/ClingingComponent/Blueprints/Components/BP_ClingObject_Base.BP_ClingObject_Base_C|GetType _array_element) Type)
      (Utilities|Array|Add _localobjects _array_element)))
  (return (LocalVariables|GetLocalObjects)))

(fn GetClosestClingObject
  (params (Attached? :type Boolean) (Location :type Vector) (Radius :type Float%20%28single-precision%29) (TraceChannel :type ETraceTypeQuery%20Enum :default "TraceTypeQuery1") (ActorsToIgnore :type Array%20of%20Actor%20Object%20References) (DrawDebugType :type EDrawDebugTrace%20Enum :default "None"))
  (bind (_outhits _returnvalue) (Collision|MultiSphereTraceByChannel 0 Location Location Radius TraceChannel false ActorsToIgnore DrawDebugType))
  (if _returnvalue
    (LocalVariables|SetLocalDistance 1e+06)
    (LocalVariables|SetLocalActor 0)
    (for _array_element _outhits
      (if (.bSuccess (Utilities|Casting|CastToBP_ClingObject_Base (.HitActor (Collision|BreakHitResult _array_element))))
        (if Attached?
          (Utilities|IsValid (Actor|GetAttachParentActor (.HitActor (Collision|BreakHitResult _array_element)))
            (:Is%20Valid
              _))
          (else
            (Utilities|IsValid (Actor|GetAttachParentActor (.HitActor (Collision|BreakHitResult _array_element)))
              (:Is%20Not%20Valid
                _))))
        (if (< (.Distance (Collision|BreakHitResult _array_element)) (LocalVariables|GetLocalDistance))
          (LocalVariables|SetLocalDistance (.Distance (Collision|BreakHitResult _array_element)))
          (LocalVariables|SetLocalActor (.HitActor (Collision|BreakHitResult _array_element))))))
    (Utilities|IsValid (LocalVariables|GetLocalActor)
      (:Is%20Valid
        (return (.AsBP%20Base%20Cling%20Object (Utilities|Casting|CastToBP_ClingObject_Base (LocalVariables|GetLocalActor))) true))
      (:Is%20Not%20Valid
        (return 0 false)))
    (else
      (return 0 false))))

(fn GetClosestClingObjectonActor
  (params (SelfTarget :type Actor%20Object%20Reference) (OtherActor :type Actor%20Object%20Reference))
  (bind _objects (CallFunction|GetAllClingObjects OtherActor))
  (if (> (Utilities|Array|Length _objects) 0)
    (LocalVariables|SetLocalDistance 1e+06)
    (for _array_element _objects
      (if (< (Transformation|GetDistanceTo SelfTarget _array_element) (LocalVariables|GetLocalDistance))
        (LocalVariables|SetLocalDistance (Transformation|GetDistanceTo SelfTarget _array_element))
        (LocalVariables|SetLocalClingObject _array_element)))
    (Utilities|IsValid (LocalVariables|GetLocalClingObject)
      (:Is%20Valid
        (return (LocalVariables|GetLocalClingObject) true))
      (:Is%20Not%20Valid
        (return 0 false)))
    (else
      (return 0 false))))

(fn GetClingMovetoActor
  (params (Object :type BP%20Cling%20Object%20Base%20Object%20Reference) (TargetActor :type Actor%20Object%20Reference))
  (return (Default|GetClosestPointonType Object (Transformation|GetActorLocation TargetActor))))

(fn GetClingMovetoLocation
  (params (Object :type BP%20Cling%20Object%20Base%20Object%20Reference) (TargetLocation :type Vector) (TargetActor :type Actor%20Object%20Reference))
  (return (Default|GetClosestPointonType Object (select (Utilities|IsValid TargetActor) (Transformation|GetActorLocation TargetActor) TargetLocation))))

(fn GetClingObjectParent
  (params (Object :type BP%20Cling%20Object%20Base%20Object%20Reference))
  (bind _returnvalue (Actor|GetParentActor Object))
  (return _returnvalue (Utilities|IsValid _returnvalue)))

(fn GetAllClingObjects
  (params (Actor :type Actor%20Object%20Reference))
  (bind _localobjects (LocalVariables|GetLocalObjects))
  (Utilities|IsValid Actor
    (:Is%20Valid
      (for _array_element (Actor|GetAllChildActors Actor true)
        (if (.bSuccess (Utilities|Casting|CastToBP_ClingObject_Base _array_element))
          (Utilities|Array|Add _localobjects (.AsBP%20Base%20Cling%20Object (Utilities|Casting|CastToBP_ClingObject_Base _array_element))))))
    (:Is%20Not%20Valid
      _))
  (return _localobjects))