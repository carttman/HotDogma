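; Companion manager that switches the active companion command from player input.
; It sets the Following command on BeginPlay, and input actions 1 to 4 select Following, Go, Wait or Help through SetCommand.
; Each switch prints its number as debug output, while the construction script, overlap and Tick events are empty.
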(event EventBeginPlay
  (Class|HDCompanionManager|SetCommand "Command_Following")
  (Development|PrintString "1"))

(event Collision|EventActorBeginOverlap
  (params (OtherActor :type Actor%20Object%20Reference)))

(event EventTick
  (params (DeltaSeconds :type Float%20%28single-precision%29)))

(event Input|ActionEvents|InputAction1
  (params (Key :type Key%20Structure :default "None"))
  (:Pressed
    (Class|HDCompanionManager|SetCommand "Command_Following")
    (Development|PrintString "1")))

(event Input|ActionEvents|InputAction2
  (params (Key :type Key%20Structure :default "None"))
  (:Pressed
    (Class|HDCompanionManager|SetCommand "Command_Go")
    (Development|PrintString "2")))

(event Input|ActionEvents|InputAction3
  (params (Key :type Key%20Structure :default "None"))
  (:Pressed
    (Class|HDCompanionManager|SetCommand "Command_Wait")
    (Development|PrintString "3")))

(event Input|ActionEvents|InputAction4
  (params (Key :type Key%20Structure :default "None"))
  (:Pressed
    (Class|HDCompanionManager|SetCommand "Command_Help")
    (Development|PrintString "4")))

(fn ConstructionScript)