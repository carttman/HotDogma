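; BP_Casting is a magic casting effect Blueprint with start, stop and cancel events.
; Start tints two Niagara systems with CastingColor and activates them, while the Casting timeline drives the second system's scale.
; Stop deactivates both and fires a particle system, whereas cancel only deactivates them.
; BeginPlay just prints a debug "Hello".
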(event Collision|EventActorBeginOverlap
  (params (OtherActor :type Actor%20Object%20Reference)))

(event EventTick
  (params (DeltaSeconds :type Float%20%28single-precision%29)))

(event EventOnCastingStart
  (params (CastingTime :type Float%20%28single-precision%29))
  (bind _niagara (Variables|Default|GetNiagara))
  (bind _castingcolor (Variables|Default|GetCastingColor))
  (bind _niagara1 (Variables|Default|GetNiagara1))
  (Niagara|SetNiagaraVariable(LinearColor) _niagara "Color01" _castingcolor)
  (Niagara|SetNiagaraVariable(LinearColor) _niagara "Color2" _castingcolor)
  (Components|Activation|Activate _niagara true)
  (Niagara|SetNiagaraVariable(LinearColor) _niagara1 "Color01" _castingcolor)
  (Niagara|SetNiagaraVariable(LinearColor) _niagara1 "Color02" _castingcolor)
  (Niagara|SetNiagaraVariable(LinearColor) _niagara1 "Color03" _castingcolor)
  (Components|Activation|Activate _niagara1 true)
  (bind _newtrack_0 (Timeline|Casting PlayFromStart)
    (:Update
      (Transformation|SetRelativeScale3D (Variables|Default|GetNiagara1) (Math|Conversions|ToVector(Float) _newtrack_0)))))

(event EventOnCastingCancel
  (Components|Activation|Deactivate (Variables|Default|GetNiagara))
  (Components|Activation|Deactivate (Variables|Default|GetNiagara1)))

(event EventOnCastingStop
  (Components|Activation|Deactivate (Variables|Default|GetNiagara))
  (Components|Activation|Deactivate (Variables|Default|GetNiagara1))
  (Components|Activation|Activate (Variables|Default|GetParticleSystem) true))

(event EventBeginPlay
  (Development|PrintString "Hello"))

(fn ConstructionScript)