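; BP_HighHagol is a magic hazard actor that deals periodic damage to HD_Dragon actors and plays a sea storm sound on spawn.
; Tick accumulates time and flips a flag at each interval, toggling the capsule's collision on and off to pulse the damage window.
; Capsule begin-overlap events with a dragon apply fixed damage and spawn a hit emitter at the actor's own location.
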(event OnComponentBeginOverlap(Capsule)
  (params (OverlappedComponent :type Primitive%20Component%20Object%20Reference) (OtherActor :type Actor%20Object%20Reference) (OtherComp :type Primitive%20Component%20Object%20Reference) (OtherBodyIndex :type Integer) (bFromSweep :type Boolean) (SweepResult :type Hit%20Result%20Structure%20%28by%20ref%29))
  (bind _ashd_dragon (Utilities|Casting|CastToHD_Dragon OtherActor))
  (Game|Damage|ApplyDamage _ashd_dragon 5.0 0 0)
  (Effects|SpawnEmitteratLocation "/Game/LGT/VFX/PS_MagicHit/P_ky_hit1.P_ky_hit1" (Transformation|GetActorLocation) (Transformation|GetActorRotation)))

(event EventBeginPlay
  (Audio|PlaySoundatLocation "/Game/Assets/SFX/Magic/AMBIENCE_Sea_Storm_01_16sec_loop_stereo.AMBIENCE_Sea_Storm_01_16sec_loop_stereo" (Transformation|GetActorLocation) "0, 0, 0" 1.0 1.0 0.0 0 0 0 0))

(event EventTick
  (params (DeltaSeconds :type Float%20%28single-precision%29))
  (bind _capsule (Variables|Default|GetCapsule))
  (bind _output_get (Variables|Default|SetcurrentTime (+ (Variables|Default|GetcurrentTime) DeltaSeconds)))
  (if (> _output_get (Variables|Default|Gettime))
    (bind _output_get_2 (Variables|Default|SetbDamage (not (Variables|Default|GetbDamage))))
    (Variables|Default|SetcurrentTime 0.0)
    (if _output_get_2
      (Collision|SetCollisionEnabled _capsule "NoCollision")
      (else
        (Collision|SetCollisionEnabled _capsule "QueryAndPhysics")))))

(fn ConstructionScript)