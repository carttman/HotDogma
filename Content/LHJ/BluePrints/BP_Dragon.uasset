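; BP_Dragon is the dragon character Blueprint, which as written only visualizes ranges from its HD_DragonFSM component.
; Every Tick it draws two flat debug circles slightly above the actor's origin: red for AttackDist and blue for ThresholdRadian, which is used as a radius.
; Unconnected leftover nodes would switch movement to Flying and push the dragon upward to TargetHeight, but they never run.
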(event EventBeginPlay)

(event Collision|EventActorBeginOverlap
  (params (OtherActor :type Actor%20Object%20Reference)))

(event EventTick
  (params (DeltaSeconds :type Float%20%28single-precision%29))
  (bind _returnvalue (Transformation|GetActorLocation))
  (bind _returnvalue_2 (Actor|GetComponentbyClass "/Script/HotDogma.HD_DragonFSM"))
  (bind _returnvalue_3 (+ (.z _returnvalue) 4e+01))
  (bind _returnvalue_4 (Math|Vector|MakeVector (.x _returnvalue) (.y _returnvalue) _returnvalue_3))
  (Rendering|Debug|DrawDebugCircle _returnvalue_4 (Variables|/Script/HotDogma.HD_DragonFSM|GetAttackDist _returnvalue_2) 12 "(R=1.000000,G=0.000000,B=0.000000,A=1.000000)" 0.0 0.0 "1.000000,0.000000,0.000000" "0.000000,1.000000,0.000000")
  (Rendering|Debug|DrawDebugCircle _returnvalue_4 (Math|Conversions|ToFloat(Integer) (Variables|/Script/HotDogma.HD_DragonFSM|GetThresholdRadian _returnvalue_2)) 12 "(R=0.000000,G=0.238182,B=1.000000,A=1.000000)" 0.0 0.0 "1.000000,0.000000,0.000000" "0.000000,1.000000,0.000000"))

(fn ConstructionScript)